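; BP_Vaultable_Object is an environment Blueprint that marks a world object as vaultable.
; It answers four capability queries with constants: Is Vaultable returns true, while Is Interactable, Is Destructable and Is Pickupable return false.
; The event graph and construction script add no logic of their own, so any vaulting behavior lives outside this Blueprint.
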(event EventBeginPlay)

(event EventTick
  (params (DeltaSeconds :type Float%20%28single-precision%29))
  (|CallParentFunction DeltaSeconds) ; This node is disabled and will not be called.\nDrag off pins to build functionality.
)

(fn ConstructionScript
  (|CallParentFunction))

(fn IsVaultable
  (return true))

(fn IsInteractable
  (return false))

(fn IsDestructable
  (return false))

(fn IsPickupable
  (return false))