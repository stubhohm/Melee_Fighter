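; Axe pickup actor that gives the player a weapon and reports itself as interactable and pickupable, but not destructable or vaultable.
; On Pickup it builds hardcoded weapon data for Escanor's axe and, for one ItemType value, adds it to BP_Player_Character's inventory system component, then destroys itself with a debug print.
; Other item types, Interact and DestroyObject have no behavior.
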(event EventBeginPlay
  (|CallParentFunction) ; This node is disabled and will not be called.\nDrag off pins to build functionality.
)

(event Collision|EventActorBeginOverlap
  (params (OtherActor :type Actor%20Object%20Reference))
  (|CallParentFunction OtherActor) ; This node is disabled and will not be called.\nDrag off pins to build functionality.
)

(event EventTick
  (params (DeltaSeconds :type Float%20%28single-precision%29))
  (|CallParentFunction DeltaSeconds) ; This node is disabled and will not be called.\nDrag off pins to build functionality.
)

(event EventDestroyObject
  (params (Interacting%20Player :type Actor%20Object%20Reference)))

(event EventInteract
  (params (Interacting%20Player :type Actor%20Object%20Reference)))

(event EventPickup
  (params (Interacting%20Player :type Actor%20Object%20Reference))
  (Variables|Default|SetInteracting%20Player Interacting%20Player)
  (Variables|Default|SetWeapon%20Data (Utilities|Struct|MakeSTX_Weapons (Variables|Default|GetWeapon%20Data%20Weapon%20Name) "/Game/Equipment/Wieldable/Axe/GI_Escanors_Axe.GI_Escanors_Axe_C" "/Engine/EditorResources/Ai_Spawnpoint.Ai_Spawnpoint" 1e+02 30 15 30 12))
  (if (Utilities|Enum|Equal(Enum) (Variables|Default|GetItem%20Type) "NewEnumerator1")
    (bind _asbp_player_character (Utilities|Casting|CastToBP_Player_Character (Variables|Default|GetInteracting%20Player)))
    (Default|AddItemtoWeapons (Variables|/Game/Player/Blueprints/BP_Player_Character.BP_Player_Character_C|GetBPC_Inventory_System _asbp_player_character) (Variables|Default|GetWeapon%20Data))
    (Actor|DestroyActor)
    (Development|PrintString "item taken")
    (elif (not (Utilities|Enum|Equal(Enum) (Variables|Default|GetItem%20Type) "NewEnumerator0"))
      (if (Utilities|Enum|Equal(Enum) (Variables|Default|GetItem%20Type) "NewEnumerator2")
        _))))

(fn ConstructionScript
  (|CallParentFunction))

(fn IsInteractable
  (return true))

(fn IsDestructable
  (return false))

(fn IsVaultable
  (return false))

(fn IsPickupable
  (return true))