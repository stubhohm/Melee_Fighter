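; BP_Interactable_Object is an environment object Blueprint that exposes an interaction interface with no behavior of its own, apparently as a base for interactable props.
; Four query functions report whether it is interactable, destructable, vaultable or pickupable, and all return false.
; The Interact and DestroyObject events are empty, the construction script only calls its parent, and BeginPlay, overlap and Tick are disabled.
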(event EventBeginPlay
  (|CallParentFunction) ; This node is disabled and will not be called.\nDrag off pins to build functionality.
)

(event Collision|EventActorBeginOverlap
  (params (OtherActor :type Actor%20Object%20Reference))
  (|CallParentFunction OtherActor) ; This node is disabled and will not be called.\nDrag off pins to build functionality.
)

(event EventTick
  (params (DeltaSeconds :type Float%20%28single-precision%29))
  (|CallParentFunction DeltaSeconds) ; This node is disabled and will not be called.\nDrag off pins to build functionality.
)

(event EventDestroyObject
  (params (Interacting%20Player :type Actor%20Object%20Reference)))

(event EventInteract
  (params (Interacting%20Player :type Actor%20Object%20Reference)))

(fn ConstructionScript
  (|CallParentFunction))

(fn IsInteractable
  (return false))

(fn IsDestructable
  (return false))

(fn IsVaultable
  (return false))

(fn IsPickupable
  (return false))