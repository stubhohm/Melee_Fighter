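; Default enemy AI controller that runs BT_Default_AI on possession and drives its blackboard state from perception.
; Sight of the player or damage triggers Aggro, while sounds set Investigating with a point of interest; only Passive or Investigating enemies react.
; Perception updates also copy attack type and the sensed actor's attack and dodge states to the blackboard through message calls.
; Enemy death sets Dead, halting sense handling.
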(event OnPerceptionUpdated(AIPerception)
  (params (UpdatedActors :type Array%20of%20Actor%20Object%20References))
  ;[0 0 0] Detect and Target
  (Utilities|FlowControl|Sequence
    (:then_0
      (CallFunction|GetOwnerValues)
      (if (not (Variables|Default|GetDead))
        (for _array_element UpdatedActors
          (Variables|Default|SetSensed%20Actor _array_element)
          (Utilities|FlowControl|Sequence
            (:then_0
              (bind _sensed (CallFunction|CanSenseActor (Variables|Default|GetSensed%20Actor) "NewEnumerator1"))
              (if _sensed
                (SenseHandling|HandleSenseSight (Variables|Default|GetSensed%20Actor))))
            (:then_1
              (bind (_sensed_2 _stimulus) (CallFunction|CanSenseActor (Variables|Default|GetSensed%20Actor) "NewEnumerator2"))
              (if _sensed_2
                (SenseHandling|HandleSenseSound (.StimulusLocation (Utilities|Struct|BreakAIStimulus _stimulus)))))
            (:then_2
              (bind _sensed_3 (CallFunction|CanSenseActor (Variables|Default|GetSensed%20Actor) "NewEnumerator3"))
              (if _sensed_3
                (SenseHandling|HandleSenseDamage (Variables|Default|GetSensed%20Actor))))))
        (else
          (StateModifying|SetStateasDead))))
    (:then_1
      (bind _enem_state (CallFunction|GetCurrentState))
      (if (Utilities|Enum|Equal(Enum) _enem_state "NewEnumerator2")
        (CallFunction|SetAttackState)))))

(event EventEnemyDied
  ;[0 0 0] Detect and Target
  (StateModifying|SetStateasDead))

(event EventPossess
  (params (PossessedPawn :type Pawn%20Object%20Reference))
  (bind _owner (Class|BPIPlayerInterface|GetOwnerRef(Message) PossessedPawn))
  (Variables|Actor|SetOwning%20Enemy%20Actor _owner)
  (AI|RunBehaviorTree "/Game/Enemy_Blue_Prints/AI_system/BT_Default_AI.BT_Default_AI")
  (StateModifying|SetStateasPassive))

(fn ConstructionScript)

(fn SetStateasPassive
  (AI|Components|Blackboard|SetValueasEnum (Variables|Default|GetBlackboard) (Variables|KeyNames|GetEnemy%20State) (Utilities|Enum|LiteralenumENUM_AI_States "NewEnumerator0")))

(fn SetStateasStunned
  (AI|Components|Blackboard|SetValueasEnum (Variables|Default|GetBlackboard) (Variables|KeyNames|GetEnemy%20State) (Utilities|Enum|LiteralenumENUM_AI_States "NewEnumerator1")))

(fn SetStateasAggro
  (params (target :type Actor%20Object%20Reference))
  (Class|BPIEnemyInterface|SetTargetRef(Message) (Pawn|GetControlledPawn) target)
  (AI|Components|Blackboard|SetValueasObject (Variables|Default|GetBlackboard) (Variables|KeyNames|GetAttack%20Target) target)
  (AI|Components|Blackboard|SetValueasEnum (Variables|Default|GetBlackboard) (Variables|KeyNames|GetEnemy%20State) (Utilities|Enum|LiteralenumENUM_AI_States "NewEnumerator2")))

(fn SetStateasDead
  (AI|Components|Blackboard|SetValueasEnum (Variables|Default|GetBlackboard) (Variables|KeyNames|GetEnemy%20State) (Utilities|Enum|LiteralenumENUM_AI_States "NewEnumerator3")))

(fn CanSenseActor
  (params (Actor :type Actor%20Object%20Reference) (Sense :type ENUM_AI_Senses%20Enum :default "NewEnumerator0"))
  (bind _info (Class|AIPerceptionComponent|GetActorsPerception (Variables|Default|GetAIPerception) Actor))
  (for _array_element (.LastSensedStimuli (Utilities|Struct|BreakActorPerceptionBlueprintInfo _info))
    (bind _returnvalue (Class|AIPerceptionSystem|GetSenseClassforStimulus _array_element))
    (if (== _returnvalue (Utilities|Select :Index Sense :NewEnumerator0 0 :NewEnumerator1 "/Script/AIModule.AISense_Sight" :NewEnumerator2 "/Script/AIModule.AISense_Hearing" :NewEnumerator3 "/Script/AIModule.AISense_Damage"))
      (return (.bSuccessfullySensed (Utilities|Struct|BreakAIStimulus _array_element)) _array_element))))

(fn HandleSenseSight
  (params (Actor :type Actor%20Object%20Reference))
  (bind _output_get (LocalVariables|SetSeen%20Actor Actor))
  (if (== _output_get (Game|GetPlayerCharacter 0))
    (bind _enem_state (CallFunction|GetCurrentState))
    (switch Utilities|FlowControl|Switch|SwitchonENUM_AI_States _enem_state
      (:NewEnumerator0
        _)
      (:NewEnumerator4
        _))
    (StateModifying|SetStateasAggro (LocalVariables|GetSeen%20Actor))))

(fn GetCurrentState
  (return (Utilities|Enum|ByteToEnumENUM_AI_States (Class|BlackboardComponent|GetValueasEnum (Variables|Default|GetBlackboard) (Variables|KeyNames|GetEnemy%20State)))))

(fn HandleSenseSound
  (params (Location :type Vector))
  (LocalVariables|SetSound%20Location Location)
  (bind _enem_state (CallFunction|GetCurrentState))
  (switch Utilities|FlowControl|Switch|SwitchonENUM_AI_States _enem_state
    (:NewEnumerator0
      _)
    (:NewEnumerator4
      _))
  (StateModifying|SetStateasInvestigating (LocalVariables|GetSound%20Location)))

(fn SetStateasInvestigating
  (params (Location :type Vector))
  (AI|Components|Blackboard|SetValueasVector (Variables|Default|GetBlackboard) (Variables|KeyNames|GetPoint%20of%20Interest) Location)
  (AI|Components|Blackboard|SetValueasEnum (Variables|Default|GetBlackboard) (Variables|KeyNames|GetEnemy%20State) (Utilities|Enum|LiteralenumENUM_AI_States "NewEnumerator4")))

(fn HandleSenseDamage
  (params (Actor :type Actor%20Object%20Reference))
  (LocalVariables|SetDamaging%20Actor Actor)
  (bind _enem_state (CallFunction|GetCurrentState))
  (switch Utilities|FlowControl|Switch|SwitchonENUM_AI_States _enem_state
    (:NewEnumerator0
      _)
    (:NewEnumerator4
      _))
  (bind _hit_points (Class|BPIEnemyInterface|GetEnemyHP,andManaPoints(Message) (Variables|Actor|GetOwning%20Enemy%20Actor)))
  (if (== _hit_points 0.0)
    (StateModifying|SetStateasDead)
    (else
      (StateModifying|SetStateasAggro (LocalVariables|GetDamaging%20Actor)))))

(fn GetOwnerValues
  (Utilities|FlowControl|Sequence
    (:then_0
      (Variables|Actor|SetOwning%20Enemy%20Actor (Pawn|GetControlledPawn))
      (bind _dead (Class|BPIAIEnemyBT|IsEnemyDead(Message) (Variables|Actor|GetOwning%20Enemy%20Actor)))
      (Variables|Default|SetDead _dead)
      (bind _attack_type (Class|BPIEnemyInterface|GetCurrentAttackType(Message) (Variables|Actor|GetOwning%20Enemy%20Actor)))
      (bind _output_get (Variables|Default|SetAttack%20Type _attack_type))
      (AI|Components|Blackboard|SetValueasEnum (Variables|Default|GetBlackboard) (Variables|KeyNames|GetCurrent%20Attack%20Type%20Key) (Utilities|Enum|LiteralenumENUM_Enemy_Attack_types _output_get)))
    (:then_1
      (bind _attack_state (Class|BPIPlayerInterface|GetAttackState(Message) (Variables|Default|GetSensed%20Actor)))
      (bind _output_get_2 (Variables|Default|SetTarget%20Attack%20State _attack_state))
      (AI|Components|Blackboard|SetValueasBool (Variables|Default|GetBlackboard) (Variables|KeyNames|GetTarget%20Attack%20State%20Key) (Class|KismetSystemLibrary|MakeLiteralBool _output_get_2))
      (bind _dodge_state (Class|BPIPlayerInterface|GetDodgeState(Message) (Variables|Default|GetSensed%20Actor)))
      (bind _output_get_3 (Variables|Default|SetTarget%20Dodge%20State _dodge_state))
      (AI|Components|Blackboard|SetValueasBool (Variables|Default|GetBlackboard) (Variables|Default|GetTarget%20Dodge%20State%20Key) (Class|KismetSystemLibrary|MakeLiteralBool _output_get_3)))))

(fn SetAttackState
  (AI|Components|Blackboard|SetValueasEnum (Variables|Default|GetBlackboard) (Variables|KeyNames|GetAttack%20Type%20Key) (Utilities|Enum|LiteralenumENUM_Enemy_Attack_types (Variables|Default|GetAttack%20Type))))