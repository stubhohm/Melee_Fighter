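; BP_Patrol_Route is a patrol path for enemy AI, defined by a spline whose points serve as waypoints.
; IncrementPatrolRoute steps CurrentIndex by Direction and loops: reaching the last point going forward resets to zero, and reaching zero in reverse jumps to the point count, one past the last valid index.
; GetSplinePointAsWorldPosition returns the current point's world location.
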(event Custom|IncrementPatrolRoute
  (Variables|Default|SetCurrent%20Index (+ (Variables|Default|GetDirection) (Variables|Default|GetCurrent%20Index)))
  (if (and (== (Variables|Default|GetCurrent%20Index) 0) (< (Variables|Default|GetDirection) 0))
    (Variables|Default|SetCurrent%20Index (Spline|GetNumberOfSplinePoints (Variables|Default|GetPatrol%20Route)))
    (elif (and (== (- (Spline|GetNumberOfSplinePoints (Variables|Default|GetPatrol%20Route)) 1) (Variables|Default|GetCurrent%20Index)) (> (Variables|Default|GetDirection) 0))
      (Variables|Default|SetCurrent%20Index 0))))

(fn ConstructionScript)

(fn GetSplinePointasWorldPosition
  (return (Spline|GetLocationatSplinePoint (Variables|Default|GetPatrol%20Route) (Variables|Default|GetCurrent%20Index) "World")))