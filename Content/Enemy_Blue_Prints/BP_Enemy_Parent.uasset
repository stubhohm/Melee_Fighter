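; Parent enemy character that handles stats, equipment, combat, health display and death for AI enemies.
; BeginPlay spawns helper actors, equips weapon and armor, then derives attack ratings from weapon scaling and a stat data table.
; Attacks spawn light or heavy ability actors, while incoming damage passes through armor, reports to AI perception and sets the target.
; Tick drives a camera-facing health bar with delayed drain and triggers ragdoll death at zero HP.
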(event EventCompleteEnemyAttack)

(event EventEnemyAttack
  (params (Attack%20Index :type Integer) (Attack%20Type :type ENUM_Enemy_Attack_types%20Enum :default "NewEnumerator4") (Combo :type Boolean) (Punish :type Boolean) (Calling%20BTT :type BT%20Task%20Blueprint%20Base%20Object%20Reference))
  (Development|PrintString (Utilities|String|Append "Index at Calling for Attack" (Utilities|String|ToString(Integer) Attack%20Index)) true true "(R=0.000000,G=0.660000,B=1.000000,A=1.000000)" 1e+01)
  (Variables|Default|SetAttack%20Index Attack%20Index)
  (bind _output_get (Variables|Default|SetCurrent%20Attack%20Type Attack%20Type))
  (Variables|Default|SetCalling%20BTT Calling%20BTT)
  (Variables|Default|SetPunish Punish)
  (Variables|Default|SetCombo Combo)
  (switch Utilities|FlowControl|Switch|SwitchonENUM_Enemy_Attack_types _output_get
    (:NewEnumerator0
      (bind _returnvalue (Game|SpawnActorfromClass "/Game/GamePlayAbilities/GA_Combat/Enemy_Combat_Abilities/GA_Enemy_Combat_Light_Attack.GA_Enemy_Combat_Light_Attack_C" (Variables|Default|GetSpawn%20Transform) "Undefined" "MultiplyWithRoot" 0 "NewEnumerator0" 0))
      (bind _output_get_2 (Variables|Default|SetActive%20Combat%20Ability _returnvalue))
      (Class|BPIEnemyCombat|InitiateLightAttack(Message) _output_get_2 self (Variables|Default|GetAttack%20Index) (Variables|Default|GetCombo) (Variables|Default|GetPunish)))
    (:NewEnumerator1
      (bind _returnvalue_2 (Game|SpawnActorfromClass "/Game/GamePlayAbilities/GA_Combat/Enemy_Combat_Abilities/GA_Enemy_Combat_Heavy_Attack.GA_Enemy_Combat_Heavy_Attack_C" (Variables|Default|GetSpawn%20Transform) "Undefined" "MultiplyWithRoot" 0 "NewEnumerator0" 0))
      (bind _output_get_3 (Variables|Default|SetActive%20Combat%20Ability _returnvalue_2))
      (Class|BPIEnemyCombat|InitiateHeavyAttack(Message) _output_get_3 self (Variables|Default|GetAttack%20Index) (Variables|Default|GetCombo) (Variables|Default|GetPunish)))))

(event EventSetTargetRef
  (params (Set%20Target%20Ref :type Actor%20Object%20Reference))
  (Variables|Refs|SetActive%20Target Set%20Target%20Ref))

(event EventSetAttackType
  (params (Current%20Attack%20Type :type ENUM_Enemy_Attack_types%20Enum :default "NewEnumerator4"))
  (Variables|Default|SetCurrent%20Attack%20Type Current%20Attack%20Type))

(event EventSetEnemyAbilityDamge
  (params (Physical%20Ability%20Damage :type Float%20%28double-precision%29) (Elemental%20Ability%20Damage :type Float%20%28double-precision%29))
  (Variables|AbilityDamage|SetPhysical%20Ability%20Damage Physical%20Ability%20Damage)
  (Variables|AbilityDamage|SetElemental%20Ability%20Damage Elemental%20Ability%20Damage))

(event EventSetEnemyAttackState
  (params (Attack%20State :type Boolean))
  (Variables|Bools|SetAttack%20State Attack%20State))

(event EventSetEnemyCrouchState
  (params (Crouch%20State :type Boolean))
  (Variables|Bools|SetCrouch%20State Crouch%20State))

(event EventSetEnemyDodgeState
  (params (Dodge%20State :type Boolean))
  (Variables|Bools|SetDodge%20State Dodge%20State))

(event EventSetEnemyBlockState
  (params (Block%20State :type Boolean))
  (Variables|Default|SetBlock%20State Block%20State))

(event EventTick
  (params (DeltaSeconds :type Float%20%28single-precision%29))
  ;[0 0 0] On Tick Events
  (Utilities|FlowControl|Sequence
    (:then_0
      (Utilities|FlowControl|DoOnce false
        (:Completed
          (HPBarDisplay|CreateWidget)
          (HPBarDisplay|HideHealthBar))))
    (:then_1
      (if (Variables|Bools|GetIs_health_visible)
        (HPBarDisplay|RotateBartoFacePlayer)
        (if (Variables|DamageCalculations|GetTook%20Damage)
          (HPBarDisplay|UpdateHealthBar)
          (Variables|DamageCalculations|SetTook%20Damage false)
          (bind _aswbp_enemy_health_bar_display (Utilities|Casting|CastToWBP_Enemy_HealthBar_Display (UserInterface|GetWidget (Variables|Default|GetHealth%20Bar%20Widget))))
          (bind _hp_decrease (Timeline|HP%20Delay PlayFromStart)
            (:Update
              (Progress|SetPercent (Variables|/Game/Enemy_Blue_Prints/Enemy_Widgets/WBP_Enemy_HealthBar_Display.WBP_Enemy_HealthBar_Display_C|GetDelayhealthBar _aswbp_enemy_health_bar_display) (/ (Math|Float|Lerp (Variables|EnemyStats|GetPrevious%20Hit%20Points) (Variables|EnemyStats|GetHit%20Points) _hp_decrease) (Variables|EnemyStats|GetMax%20Hit%20Points))))))))
    (:then_2
      (if (<= (Variables|EnemyStats|GetHit%20Points) 0.0)
        (Damage|EnemyDeath)))))

(event EventSetEnemySprintState
  (params (Sprint%20State :type Boolean))
  (Variables|Bools|SetSprint%20State Sprint%20State))

(event EventInitEnemyActor
  ;[0 0 0] Init Enemy Enemy
  (Utilities|FlowControl|DoOnce true) ; enters at Reset
)

(event EventEnemyTakeDamage
  (params (Attacker :type Actor%20Object%20Reference) (Attacked :type Actor%20Object%20Reference) (Physical%20Damage%20Type :type ENUM_Damage_Type%20Enum :default "NewEnumerator0") (Physcial%20Damage :type Float%20%28double-precision%29) (Element%20Damage%20Type :type ENUM_Element_Type%20Enum :default "NewEnumerator0") (Elemental%20Damage :type Float%20%28double-precision%29))
  (bind _self self)
  ;[0 0 0] Take Damage Event
  (Variables|Refs|SetAttacker%20Ref Attacker)
  (Utilities|FlowControl|Sequence
    (:then_0
      (Damage|CalculatePhyscialDamage Physical%20Damage%20Type Physcial%20Damage))
    (:then_1
      (Damage|CalculateElementalDamage Element%20Damage%20Type Elemental%20Damage))
    (:then_2
      (Variables|EnemyStats|SetPrevious%20Hit%20Points (Variables|EnemyStats|GetHit%20Points))
      (Variables|EnemyStats|SetHit%20Points (Utilities|Operators|Subtract (Variables|EnemyStats|GetHit%20Points) (Variables|DamageCalculations|GetPhyscial%20Damage) (Variables|DamageCalculations|GetElemental%20Damage)))
      (Variables|DamageCalculations|SetTook%20Damage true)
      (Utilities|FlowControl|DoOnce false
        (:Completed
          (HPBarDisplay|DisplayHealthBar)
          (Utilities|FlowControl|Sequence
            (:then_0
              (Variables|AI|SetTarget_found true)
              (Class|AISenseDamage|ReportDamageEvent _self (Variables|Refs|GetAttacker%20Ref) (+ (Variables|DamageCalculations|GetPhyscial%20Damage) (Variables|DamageCalculations|GetElemental%20Damage)) (Transformation|GetActorLocation _self) "0, 0, 0" "None"))
            (:then_1
              (Variables|Refs|SetActive%20Target (Variables|Refs|GetAttacker%20Ref)))))))))

(event EventCallEnemyEndWeaponTrace
  (Class|BPIPlayerCombat|RelayEndWeaponTrace(Message) (Variables|Refs|GetCombat%20Parent%20Ref)))

(event EventCallEnemyStartWeaponTrace
  (params (Animation :type Anim%20Sequence%20Base%20Object%20Reference))
  (Class|BPIPlayerCombat|RelayStartWeaponTrace(Message) (Variables|Refs|GetCombat%20Parent%20Ref) self Animation (Variables|Refs|GetEnemy%20Weapon%20Ref)))

(event EventEndPlay
  (params (EndPlayReason :type EEndPlayReason%20Enum :default "Destroyed"))
  ;[0 0 0] Init Enemy Enemy
)

(event EventBeginPlay
  ;[0 0 0] Init Enemy Enemy
  (Utilities|FlowControl|DoOnce true
    (:Completed
      (Utilities|FlowControl|Sequence
        (:then_0
          (InitEnemy|SetEnemyStats))
        (:then_1
          (InitEnemy|InitSpawnerandAbilitySet)
          (InitEnemy|EquipEnemy "Da Axe" "/Game/Equipment/Wearable/GI_Test_Armor.GI_Test_Armor_C")
          (AttackRatingCalcs|SetEnemyAttackRatings))))))

(event EventCanCombo
  (Development|PrintString "Can combo" true true "(R=0.000000,G=0.660000,B=1.000000,A=1.000000)" 1e+01)
  (Class|BPICalltoAIBT|EndEnemyAttack(Message) (Variables|Default|GetCalling%20BTT)))

(event EventSetAttackIndex
  (params (Attack%20Index :type Integer))
  (Development|PrintString (Utilities|String|Append "Setting Attack Index" (Utilities|String|ToString(Integer) Attack%20Index)) true true "(R=0.000000,G=0.660000,B=1.000000,A=1.000000)" 1e+01)
  (Variables|Default|SetAttack%20Index Attack%20Index))

(fn ConstructionScript
  (|CallParentFunction))

(fn DisplayHealthBar
  (bind _output_get (Variables|Bools|SetIs_health_visible true))
  (Rendering|SetVisibility (Variables|Default|GetHealth%20Bar%20Widget) _output_get false))

(fn HideHealthBar
  (bind _output_get (Variables|Bools|SetIs_health_visible false))
  (Rendering|SetVisibility (Variables|Default|GetHealth%20Bar%20Widget) _output_get false))

(fn UpdateHealthBar
  (bind _aswbp_enemy_health_bar_display (Utilities|Casting|CastToWBP_Enemy_HealthBar_Display (UserInterface|GetWidget (Variables|Default|GetHealth%20Bar%20Widget))))
  (Progress|SetPercent (Variables|/Game/Enemy_Blue_Prints/Enemy_Widgets/WBP_Enemy_HealthBar_Display.WBP_Enemy_HealthBar_Display_C|GetEnemyHealthBar _aswbp_enemy_health_bar_display) (/ (Variables|EnemyStats|GetHit%20Points) (Variables|EnemyStats|GetMax%20Hit%20Points))))

(fn CreateWidget
  (bind _returnvalue (UserInterface|CreateWidget "/Game/Enemy_Blue_Prints/Enemy_Widgets/WBP_Enemy_HealthBar_Display.WBP_Enemy_HealthBar_Display_C"))
  (Variables|Refs|SetEnemy%20Health%20Display _returnvalue))

(fn CalculateElementalDamage
  (params (Element%20Damage%20Type :type ENUM_Element_Type%20Enum :default "NewEnumerator0") (Element%20Damage%20Dealt :type Float%20%28double-precision%29))
  (bind _elemental_damage_recieved (Class|BPIArmor|ElementalDamageReduction(Message) (Variables|Refs|GetEnemy%20Armor%20Ref) Element%20Damage%20Dealt Element%20Damage%20Type))
  (Variables|DamageCalculations|SetElemental%20Damage _elemental_damage_recieved))

(fn CalculatePhyscialDamage
  (params (Physical%20Damage%20Type :type ENUM_Damage_Type%20Enum :default "NewEnumerator0") (Physical%20Damage%20Dealt :type Float%20%28double-precision%29))
  (bind _physical_damage_recieved (Class|BPIArmor|PhyscialDamageReduction(Message) (Variables|Refs|GetEnemy%20Armor%20Ref) Physical%20Damage%20Dealt Physical%20Damage%20Type))
  (Variables|DamageCalculations|SetPhyscial%20Damage _physical_damage_recieved))

(fn RotateBartoFacePlayer
  (bind _health_bar_widget (Variables|Default|GetHealth%20Bar%20Widget))
  (Transformation|SetWorldRotation _health_bar_widget (Math|Rotator|FindLookatRotation (Transformation|GetWorldLocation _health_bar_widget) (Transformation|GetWorldLocation (Variables|/Script/Engine.PlayerCameraManager|GetTransformComponent (Game|GetPlayerCameraManager 0)))) false false))

(fn EquipEnemy
  (params (Equipped%20Weapon :type Name) (Equipped%20Armor :type GI%20Wearable%20Item%20Class%20Reference))
  (LocalVariables|SetEnemy%20Armor Equipped%20Armor)
  (InitEnemy|EquipWeapon Equipped%20Weapon)
  (bind _returnvalue (Game|SpawnActorfromClass (LocalVariables|GetEnemy%20Armor) (Transformation|GetSocketTransform (Variables|Character|GetMesh self) (Variables|Refs|GetArmor%20Socket) "RTS_World") "Undefined" "MultiplyWithRoot" 0 "NewEnumerator0" 0))
  (bind _output_get (Variables|Refs|SetEnemy%20Armor%20Ref _returnvalue))
  (Transformation|AttachComponentToComponent _output_get (Variables|Character|GetMesh self) (Variables|Refs|GetArmor%20Socket) "SnapToTarget" "SnapToTarget" "SnapToTarget" true)
  (Class|BPIWeapons|InitWeapon(Message) (Variables|Refs|GetEnemy%20Weapon%20Ref)))

(fn SetEnemyStats
  (Variables|EnemyStats|SetHit%20Points (Variables|EnemyStats|GetMax%20Hit%20Points))
  (Variables|/Script/Engine.CharacterMovementComponent|SetMaxWalkSpeed (Variables|Character|GetCharacterMovement) 1.5e+02))

(fn InitSpawnerandAbilitySet
  (Variables|Default|SetTransform (Transformation|GetActorTransform))
  (Utilities|FlowControl|Sequence
    (:then_0
      ;[0 0 0] Attack References
      (bind _returnvalue (Game|SpawnActorfromClass "/Game/GamePlayAbilities/GA_Base_Ability.GA_Base_Ability_C" (Variables|Default|GetTransform) "Undefined" "MultiplyWithRoot" 0 0))
      (Variables|Refs|SetAbility%20Ref _returnvalue))
    (:then_1
      (bind _returnvalue_2 (Game|SpawnActorfromClass :Class "/Game/Equipment/Wieldable/GI_Equiped_Weapon.GI_Equiped_Weapon_C" :SpawnTransform (Variables|Default|GetTransform) :CollisionHandlingOverride "AlwaysSpawn" :TransformScaleMethod "MultiplyWithRoot" :Instigator 0))
      (Variables|Refs|SetWeapon%20Spawner%20Ref _returnvalue_2))
    (:then_2
      (bind _returnvalue_3 (Game|SpawnActorfromClass "/Game/GamePlayAbilities/GA_Combat/Enemy_Combat_Abilities/GA_Enemy_Combat_Parent.GA_Enemy_Combat_Parent_C" (Variables|Default|GetTransform) "AlwaysSpawn" "MultiplyWithRoot" 0 "NewEnumerator0" 0))
      (Variables|Refs|SetCombat%20Parent%20Ref _returnvalue_3))))

(fn EquipWeapon
  (params (Equipped%20Weapon%20Name :type Name))
  (Variables|Refs|SetEquipped%20Weapon%20Name Equipped%20Weapon%20Name)
  (bind _weapon_actor_ref (Class|BPIWeapons|SpawnActiveWeapon(Message) (Variables|Refs|GetWeapon%20Spawner%20Ref) (Transformation|GetSocketTransform (Variables|Character|GetMesh) (Variables|Refs|GetRight%20Hand%20Socket) "RTS_World") (Variables|Refs|GetEquipped%20Weapon%20Name)))
  (bind _output_get (Variables|Refs|SetEnemy%20Weapon%20Ref _weapon_actor_ref))
  (Transformation|AttachComponentToComponent _output_get (Variables|Character|GetMesh) (Variables|Refs|GetRight%20Hand%20Socket) "SnapToTarget" "SnapToTarget" "SnapToTarget" true)
  (Class|BPIWeapons|InitWeapon(Message) (Variables|Refs|GetEnemy%20Weapon%20Ref)))

(fn CleanUpItems
  (Utilities|FlowControl|Sequence
    (:then_0
      (bind _ability_ref (Variables|Refs|GetAbility%20Ref)
        (:then
          _)
        (:else)))
    (:then_1
      (bind _active_combat_ability (Variables|Default|GetActive%20Combat%20Ability)
        (:then
          _)
        (:else)))
    (:then_2
      (bind _enemy_weapon_ref (Variables|Refs|GetEnemy%20Weapon%20Ref)
        (:then
          _)
        (:else)))
    (:then_3
      (bind _weapon_spawner_ref (Variables|Refs|GetWeapon%20Spawner%20Ref)
        (:then
          _)
        (:else)))
    (:then_4
      (bind _enemy_armor_ref (Variables|Refs|GetEnemy%20Armor%20Ref)
        (:then
          _)
        (:else))))
  (Actor|DestroyActor _ability_ref))

(fn GetWeaponScalingARs
  (bind _weapon_scaling_array (Class|BPIWeapons|GetWeaponScalingArray(Message) (Variables|Refs|GetEnemy%20Weapon%20Ref)))
  (Utilities|FlowControl|Sequence
    (:then_0
      (Variables|AttackRatingCalcs|SetStr%20Scale (Utilities|Array|Get(acopy) _weapon_scaling_array)))
    (:then_1
      (Variables|AttackRatingCalcs|SetDex%20Scale (Utilities|Array|Get(acopy) _weapon_scaling_array 1)))
    (:then_2
      (Variables|AttackRatingCalcs|SetInt%20Scale (Utilities|Array|Get(acopy) _weapon_scaling_array 2)))
    (:then_3
      (Variables|AttackRatingCalcs|SetFaith%20Scale (Utilities|Array|Get(acopy) _weapon_scaling_array 3))
      (Utilities|FlowControl|Sequence
        (:then_0
          (bind _returnvalue (Utilities|GetDataTableRow "/Game/Equipment/Wieldable/DT_Scaling_Table.DT_Scaling_Table" (Utilities|String|StringToName (Utilities|String|ToString(Integer) (Variables|Stats|GetStrength))))
            (:then
              (Variables|AttackRatingCalcs|SetStr%20Base%20AR (.damgevalue _returnvalue)))))
        (:then_1
          (bind _returnvalue_2 (Utilities|GetDataTableRow "/Game/Equipment/Wieldable/DT_Scaling_Table.DT_Scaling_Table" (Utilities|String|StringToName (Utilities|String|ToString(Integer) (Variables|Stats|GetDexterity))))
            (:then
              (Variables|AttackRatingCalcs|SetDex%20Base%20AR (.damgevalue _returnvalue_2)))))
        (:then_2
          (bind _returnvalue_3 (Utilities|GetDataTableRow "/Game/Equipment/Wieldable/DT_Scaling_Table.DT_Scaling_Table" (Utilities|String|StringToName (Utilities|String|ToString(Integer) (Variables|Stats|GetFaith))))
            (:then
              (Variables|AttackRatingCalcs|SetInt%20Base%20AR (.damgevalue _returnvalue_3)))))
        (:then_3
          (bind _returnvalue_4 (Utilities|GetDataTableRow "/Game/Equipment/Wieldable/DT_Scaling_Table.DT_Scaling_Table" (Utilities|String|StringToName (Utilities|String|ToString(Integer) (Variables|Stats|GetIntelligence))))
            (:then
              (Variables|AttackRatingCalcs|SetFaith%20Base%20AR (.damgevalue _returnvalue_4)))))))))

(fn SetEnemyAttackRatings
  (AttackRatingCalcs|GetWeaponScalingARs)
  (bind (_physical_damage _elemental_damage) (Class|BPIWeapons|GetWeaponDamage(Message) (Variables|Refs|GetEnemy%20Weapon%20Ref)))
  (bind _output_get (Variables|AttackRatingCalcs|SetTotal%20Attack%20Rating (+ (* (Variables|AttackRatingCalcs|GetStr%20Base%20AR) (Variables|AttackRatingCalcs|GetStr%20Scale)) (* (Variables|AttackRatingCalcs|GetDex%20Base%20AR) (Variables|AttackRatingCalcs|GetDex%20Scale)) (* (Variables|AttackRatingCalcs|GetInt%20Base%20AR) (Variables|AttackRatingCalcs|GetInt%20Scale)) (* (Variables|AttackRatingCalcs|GetFaith%20Base%20AR) (Variables|AttackRatingCalcs|GetFaith%20Scale)))))
  (bind _output_get_2 (Variables|AttackingCalculations|SetElemental%20Attack%20Rating (* _output_get (/ _elemental_damage _physical_damage))))
  (Variables|AttackingCalculations|SetPhysical%20Attack%20Rating (- (Variables|AttackRatingCalcs|GetTotal%20Attack%20Rating) _output_get_2)))

(fn EnemyDeath
  (Physics|SetSimulatePhysics (Variables|Character|GetMesh) true)
  (HPBarDisplay|HideHealthBar)
  (Collision|SetCollisionEnabled (Variables|Collision|GetCapsuleComponent) "NoCollision")
  (Class|BPIEnemyInterface|CallEnemyEndWeaponTrace(Message) (Variables|Refs|GetCombat%20Parent%20Ref))
  (Class|BPICalltoAIBT|EnemyDied(Message) (Pawn|GetController)))

(fn GetCurrentAttackType
  (return (Variables|Default|GetCurrent%20Attack%20Type)))

(fn GetEnemyAttackState
  (return (Variables|Bools|GetAttack%20State)))

(fn GetEnemyDodgeState
  (return (Variables|Bools|GetDodge%20State)))

(fn GetEnemyMovementComponent
  (return (Variables|Character|GetCharacterMovement)))

(fn GetEnemySprintState
  (return (Variables|Bools|GetSprint%20State)))

(fn GetEnemyAbilityDamage
  (return (Variables|AbilityDamage|GetPhysical%20Ability%20Damage) (Variables|AbilityDamage|GetElemental%20Ability%20Damage)))

(fn GetEnemyAttackIndex
  (bind _attack_index (Variables|Default|GetAttack%20Index))
  (Development|PrintString (Utilities|String|Append "Get Attacker Index " (Utilities|String|ToString(Integer) _attack_index)) true true "(R=0.000000,G=0.660000,B=1.000000,A=1.000000)" 1e+01)
  (return _attack_index))

(fn GetEnemyAttackRatings
  (return (Variables|AttackingCalculations|GetPhysical%20Attack%20Rating) (Variables|AttackingCalculations|GetElemental%20Attack%20Rating)))

(fn GetEnemyCrouchStae
  (return (Variables|Bools|GetCrouch%20State)))

(fn GetEnemyHP,andManaPoints
  (return (Variables|EnemyStats|GetHit%20Points) (Variables|Stats|GetMana%20Points)))

(fn GetEnemyMaxStats
  (return (Variables|EnemyStats|GetMax%20Hit%20Points) 0.0 (Variables|Stats|GetMax%20Mana) (Variables|Stats|GetStrength) (Variables|Stats|GetDexterity) (Variables|Stats|GetFaith) (Variables|Stats|GetIntelligence)))

(fn GetEnemyOwnerMesh
  (return (Variables|Character|GetMesh)))

(fn GetEnemyRelativeMovementDirection
  (return ""))

(fn GetEnemyWeaponRef
  (return (Variables|Refs|GetEnemy%20Weapon%20Ref)))

(fn GetOwnerEnemyRef
  (return self))

(fn GetPatrolRoute
  (Variables|Bools|Setis_patroling true)
  (return (Variables|AI|GetPatrol%20Route)))

(fn GetPatrolState
  (return false))

(fn GetTargetRef
  (return (Variables|Refs|GetActive%20Target)))

(fn IsEnemy
  (return (Variables|Bools|Getis_Enemy)))

(fn IsEnemyDead
  (return (<= (Variables|EnemyStats|GetHit%20Points) 0.0)))

(fn ReportLockon
  (params (Locked%20on :type Boolean))
  (return))

(fn SetPatrolling
  (params (is_patrolling :type Boolean))
  (bind _output_get (Variables|Bools|Setis_patroling is_patrolling))
  (return _output_get))

(fn SpeedSelection
  (params (Speed :type ENUM_Movement_Speed%20Enum :default "NewEnumerator0"))
  (bind _output_get (Variables|/Script/Engine.CharacterMovementComponent|SetMaxWalkSpeed (Variables|Character|GetCharacterMovement) (Utilities|Select :Index Speed :NewEnumerator0 0.0 :NewEnumerator1 1.5e+02 :NewEnumerator2 3.5e+02 :NewEnumerator3 5e+02)))
  (return _output_get))