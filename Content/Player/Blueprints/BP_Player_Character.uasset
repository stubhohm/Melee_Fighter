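; Player character Blueprint that turns Enhanced Input actions into combat and movement abilities and tracks health, mana and stamina.
; Init sets max stats from level-to-stat data table lookups.
; Actions gated by CanAct spawn GA_ ability actors for attacks, parry, dodge and sprint; light and heavy attacks spend stamina.
; Heavy attack starts a looping timer, apparently for stamina recharge; walk and item inputs are empty, and lock-on only stores a flag.
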(event Custom|init_player
  (bind (_max_hp _max_stamina_points _max_mana_points) (CallFunction|CalculatePlayerStats (Variables|ConstantStats|GetStat%20Array)))
  (Utilities|DefineStats _max_hp _max_stamina_points _max_mana_points)
  (Development|PrintString "Hello"))

(event Input|EnhancedActionEvents|EnhancedInputActionIA_Heavy_attack_Player
  (params (ActionValue :type Boolean) (ElapsedSeconds :type Float%20%28double-precision%29) (TriggeredSeconds :type Float%20%28double-precision%29) (InputAction :type Input%20Action%20Object%20Reference :default "/Game/Player/Inputs/Actions/Combat/IA_Heavy_attack_Player.IA_Heavy_attack_Player"))
  (Utilities|CanAct
    (:Return
      (bind _new_stamina (CallFunction|SpendStamina (Variables|MutableStats|GetStamina_Points) 3e+01))
      (Variables|MutableStats|SetStamina_Points _new_stamina)
      (Variables|ActionBools|SetIs_attacking true)
      (bind _returnvalue (Game|SpawnActorfromClass "/Game/GamePlayAbilities/GA_Combat/GA_Heavy_Attack.GA_Heavy_Attack_C" (Transformation|GetActorTransform) "Undefined" "MultiplyWithRoot" 0 "NewEnumerator0" 0.0 "NewEnumerator0" 0))
      (Default|ActivateHeavyAttack _returnvalue)
      (Variables|ActionBools|SetIs_attacking false)
      (Development|PrintString "finished attacking")
      (bind _returnvalue_2 (Utilities|Time|SetTimerbyFunctionName 0 (Variables|Default|GetFunction%20Name) 1.0 true 1.25))
      (Variables|Default|SetStamina%20Timer _returnvalue_2)
      (Development|PrintString "finished timer"))))

(event Input|EnhancedActionEvents|EnhancedInputActionIA_Light_Attack_Player
  (params (ActionValue :type Boolean) (ElapsedSeconds :type Float%20%28double-precision%29) (TriggeredSeconds :type Float%20%28double-precision%29) (InputAction :type Input%20Action%20Object%20Reference :default "/Game/Player/Inputs/Actions/Combat/IA_Light_Attack_Player.IA_Light_Attack_Player"))
  (Utilities|CanAct
    (:Return
      (bind _new_stamina (CallFunction|SpendStamina (Variables|MutableStats|GetStamina_Points) 18.0))
      (Variables|MutableStats|SetStamina_Points _new_stamina)
      (Variables|ActionBools|SetIs_attacking true)
      (bind _returnvalue (Game|SpawnActorfromClass "/Game/GamePlayAbilities/GA_Combat/GA_Light_Attack.GA_Light_Attack_C" (Transformation|GetActorTransform) "Undefined" "MultiplyWithRoot" 0 "NewEnumerator1" 0.0 "NewEnumerator0" 0))
      (Default|StartLightAttack _returnvalue))))

(event Input|EnhancedActionEvents|EnhancedInputActionIA_Dodge_Player
  (params (ActionValue :type Boolean) (ElapsedSeconds :type Float%20%28double-precision%29) (TriggeredSeconds :type Float%20%28double-precision%29) (InputAction :type Input%20Action%20Object%20Reference :default "/Game/Player/Inputs/Actions/Movement/IA_Dodge_Player.IA_Dodge_Player"))
  (Utilities|CanAct
    (:Return
      (bind _returnvalue (Game|SpawnActorfromClass "/Game/GamePlayAbilities/GA_Movement/GA_Dodge.GA_Dodge_C" (Transformation|GetActorTransform) "Undefined" "MultiplyWithRoot" 0 "NewEnumerator0" 0.0 "NewEnumerator0" 0))
      (Default|BeginDodge _returnvalue))))

(event Input|EnhancedActionEvents|EnhancedInputActionIA_Lockon_Player1
  (params (ActionValue :type Boolean) (ElapsedSeconds :type Float%20%28double-precision%29) (TriggeredSeconds :type Float%20%28double-precision%29) (InputAction :type Input%20Action%20Object%20Reference :default "/Game/Player/Inputs/Actions/CameraControl/IA_Lockon_Player1.IA_Lockon_Player1"))
  (Variables|ActionBools|SetIs_locked%20on ActionValue))

(event Input|EnhancedActionEvents|EnhancedInputActionIA_Navigate_Item_Player
  (params (ActionValue :type Vector%202D%20Structure) (ElapsedSeconds :type Float%20%28double-precision%29) (TriggeredSeconds :type Float%20%28double-precision%29) (InputAction :type Input%20Action%20Object%20Reference :default "/Game/Player/Inputs/Actions/AttributeChanges/IA_Navigate_Item_Player.IA_Navigate_Item_Player")))

(event Input|EnhancedActionEvents|EnhancedInputActionIA_Parry_Player
  (params (ActionValue :type Boolean) (ElapsedSeconds :type Float%20%28double-precision%29) (TriggeredSeconds :type Float%20%28double-precision%29) (InputAction :type Input%20Action%20Object%20Reference :default "/Game/Player/Inputs/Actions/Combat/IA_Parry_Player.IA_Parry_Player"))
  (Utilities|CanAct
    (:Return
      (Game|SpawnActorfromClass "/Game/GamePlayAbilities/GA_Combat/GA_Parry.GA_Parry_C" (Transformation|GetActorTransform) "Undefined" "MultiplyWithRoot" 0 "NewEnumerator4" 0.0 "NewEnumerator0" 0))))

(event Input|EnhancedActionEvents|EnhancedInputActionIA_Sprint_Player
  (params (ActionValue :type Vector%202D%20Structure) (ElapsedSeconds :type Float%20%28double-precision%29) (TriggeredSeconds :type Float%20%28double-precision%29) (InputAction :type Input%20Action%20Object%20Reference :default "/Game/Player/Inputs/Actions/Movement/IA_Sprint_Player.IA_Sprint_Player"))
  (Utilities|CanAct
    (:Return
      (bind _returnvalue (Game|SpawnActorfromClass "/Game/GamePlayAbilities/GA_Movement/GA_Sprint.GA_Sprint_C" (Transformation|GetActorTransform) "Undefined" "MultiplyWithRoot" 0 "NewEnumerator1" 0.0 "NewEnumerator2" 0))
      (Default|StartSprint _returnvalue (Variables|Default|GetAction%20Value%20X) (Variables|Default|GetAction%20Value%20Y) (Variables|MutableStats|GetStamina_Points)))))

(event Input|EnhancedActionEvents|EnhancedInputActionIA_Special_Attack_Player
  (params (ActionValue :type Boolean) (ElapsedSeconds :type Float%20%28double-precision%29) (TriggeredSeconds :type Float%20%28double-precision%29) (InputAction :type Input%20Action%20Object%20Reference :default "/Game/Player/Inputs/Actions/Combat/IA_Special_Attack_Player.IA_Special_Attack_Player"))
  (Utilities|CanAct
    (:Return
      (Game|SpawnActorfromClass "/Game/GamePlayAbilities/GA_Combat/GA_Special_Attack.GA_Special_Attack_C" (Transformation|GetActorTransform) "Undefined" "MultiplyWithRoot" 0 "NewEnumerator2" 0.0 "NewEnumerator0" 0))))

(event Input|EnhancedActionEvents|EnhancedInputActionIA_Use_Item_Player
  (params (ActionValue :type Boolean) (ElapsedSeconds :type Float%20%28double-precision%29) (TriggeredSeconds :type Float%20%28double-precision%29) (InputAction :type Input%20Action%20Object%20Reference :default "/Game/Player/Inputs/Actions/AttributeChanges/IA_Use_Item_Player.IA_Use_Item_Player")))

(event Input|EnhancedActionEvents|EnhancedInputActionIA_Walk_Player
  (params (ActionValue :type Vector%202D%20Structure) (ElapsedSeconds :type Float%20%28double-precision%29) (TriggeredSeconds :type Float%20%28double-precision%29) (InputAction :type Input%20Action%20Object%20Reference :default "/Game/Player/Inputs/Actions/Movement/IA_Walk_Player.IA_Walk_Player")))

(fn ConstructionScript
  (|CallParentFunction))

(fn SpendStamina
  (params (Current%20Stamina :type Float%20%28double-precision%29) (Stamina%20Cost :type Float%20%28double-precision%29))
  (if (> Current%20Stamina 0.0)
    (if (< (- (Variables|MutableStats|GetStamina_Points) Stamina%20Cost) 0.0)
      (Variables|MutableStats|SetStamina_Points 0.0)
      (else
        (Variables|MutableStats|SetStamina_Points (- (Variables|MutableStats|GetStamina_Points) Stamina%20Cost))))
    (return (Variables|MutableStats|GetStamina_Points))
    (else
      (Development|PrintString "no stamina, cannot attack"))))

(fn RechargeStamina
  (Development|PrintString "starting recharge")
  (if (and (Variables|ActionBools|GetAvailable%20to%20Act) (< (Variables|MutableStats|GetStamina_Points) (Variables|ConstantStats|GetMax_Stamina_Points)))
    (bind _output_get (Variables|MutableStats|SetStamina_Points (+ (Variables|MutableStats|GetStamina_Points) 1.0)))
    (Development|PrintString (Utilities|String|ToString(Float) _output_get))
    (Development|PrintString (Utilities|String|Append "Is Attacking" (Utilities|String|ToString(Boolean) (Variables|ActionBools|GetIs_attacking))))
    (else
      (Utilities|Time|PauseTimerbyHandle (Variables|Default|GetStamina%20Timer))
      (Development|PrintString "broke recharge"))))

(fn CalculatePlayerStats
  (params (Stat%20Array :type Array%20of%20Integers))
  (Utilities|FlowControl|Sequence
    (:then_0
      (bind _outrownames (DataTable|GetDataTableRowNames "/Game/Player/Stats/DT_Level_to_statpoints.DT_Level_to_statpoints"))
      (bind _returnvalue (Utilities|GetDataTableRow "/Game/Player/Stats/DT_Level_to_statpoints.DT_Level_to_statpoints" (Utilities|Array|Get(acopy) _outrownames (Utilities|Array|Get(acopy) Stat%20Array)))))
    (:then_1
      (bind _outrownames_2 (DataTable|GetDataTableRowNames "/Game/Player/Stats/DT_Level_to_statpoints.DT_Level_to_statpoints"))
      (bind _returnvalue_2 (Utilities|GetDataTableRow "/Game/Player/Stats/DT_Level_to_statpoints.DT_Level_to_statpoints" (Utilities|Array|Get(acopy) _outrownames_2 (Utilities|Array|Get(acopy) Stat%20Array 1)))))
    (:then_2
      (bind _outrownames_3 (DataTable|GetDataTableRowNames "/Game/Player/Stats/DT_Level_to_statpoints.DT_Level_to_statpoints"))
      (bind _returnvalue_3 (Utilities|GetDataTableRow "/Game/Player/Stats/DT_Level_to_statpoints.DT_Level_to_statpoints" (Utilities|Array|Get(acopy) _outrownames_3 (Utilities|Array|Get(acopy) Stat%20Array 2)))
        (:then
          (return (Math|Conversions|ToFloat(Integer) (.HP_Value (Utilities|Struct|BreakSTX_Level_to_statpoints _returnvalue))) (Math|Conversions|ToFloat(Integer) (.Stamina_Value (Utilities|Struct|BreakSTX_Level_to_statpoints _returnvalue_2))) (Math|Conversions|ToFloat(Integer) (.Mana_Value (Utilities|Struct|BreakSTX_Level_to_statpoints _returnvalue_3)))))))))