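; Player inventory component that handles item pickup, weapon slots, weapon equipping and the equipment menu.
; The interact input sphere-traces ahead of the owner for WorldDynamic objects and sends a pickup message to hits that are interactable and pickupable.
; The menu input toggles the equipment widget and mouse cursor.
; EquipWeapon has the owner's weapon spawner create the named weapon, then snaps it to the mesh socket, using interface messages rather than casts.
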(event Input|EnhancedActionEvents|EnhancedInputActionIA_Interact
  (params (ActionValue :type Boolean) (ElapsedSeconds :type Float%20%28double-precision%29) (TriggeredSeconds :type Float%20%28double-precision%29) (InputAction :type Input%20Action%20Object%20Reference :default "/Game/Player/Inputs/Actions/IA_Interact.IA_Interact"))
  (bind _owner (Variables|Default|GetOwner))
  (Utilities|IsValid _owner
    (:Is%20Valid
      (bind _movement_component (Class|BPIPlayerInterface|GetMovementComponent(Message) _owner))
      (bind (_outhit _returnvalue) (Collision|SphereTraceForObjects (+ (Transformation|GetActorLocation _owner) (* (Math|Vector|GetForwardVector (Variables|/Script/Engine.MovementComponent|GetUpdatedPrimitive _movement_component)) 50)) (+ (+ (Transformation|GetActorLocation _owner) (* (Math|Vector|GetForwardVector (Variables|/Script/Engine.MovementComponent|GetUpdatedPrimitive _movement_component)) 50)) (* (Math|Vector|GetForwardVector (Variables|/Script/Engine.MovementComponent|GetUpdatedPrimitive _movement_component)) 50)) 1e+02 (Utilities|Array|MakeArray "ObjectTypeQuery2") false 0 "ForDuration"))
      (if _returnvalue
        (bind _output_get (Variables|Default|SetHit%20Actor (.HitActor (Collision|BreakHitResult _outhit))))
        (bind _is_interactable (Class|BPIEnviromentalInteractions|IsInteractable(Message) _output_get))
        (if _is_interactable
          (bind _pick_upable (Class|BPIEnviromentalInteractions|IsPickupable(Message) (Variables|Default|GetHit%20Actor)))
          (if _pick_upable
            (Class|BPIEnviromentalInteractions|Pickup(Message) (Variables|Default|GetHit%20Actor) (Variables|Default|GetOwner))))))))

(event Input|EnhancedActionEvents|EnhancedInputActionIA_Toggle_Menu_HUD
  (params (ActionValue :type Boolean) (ElapsedSeconds :type Float%20%28double-precision%29) (TriggeredSeconds :type Float%20%28double-precision%29) (InputAction :type Input%20Action%20Object%20Reference :default "/Game/Player/Inputs/Actions/CameraControl/IA_Toggle_Menu_HUD.IA_Toggle_Menu_HUD"))
  (bind _returnvalue (Game|GetPlayerController 0))
  ;[0 0 0] Toggle Menu
  (bind _owner (Class|BPIPlayerInterface|GetOwnerRef(Message) (Game|GetPlayerCharacter 0)))
  (bind _output_get (Variables|Default|SetOwner _owner))
  (Utilities|IsValid _output_get
    (:Is%20Valid
      (if (Variables|Default|GetIs%20Menu%20Open)
        (Variables|Default|SetIs%20Menu%20Open false)
        (bind _equipment_widget_ref (Variables|Default|GetEquipment%20Widget%20Ref)
          (:then
            (Widget|RemovefromParent _equipment_widget_ref)
            (Variables|/Script/Engine.PlayerController|SetbShowMouseCursor _returnvalue false)
            (Input|SetInputModeGameOnly _returnvalue false))
          (:else))
        (else
          (Variables|Default|SetIs%20Menu%20Open true)
          (bind _returnvalue_2 (UserInterface|CreateWidget "/Game/UI/WB_Equipment_Menu.WB_Equipment_Menu_C"))
          (bind _output_get_2 (Variables|Default|SetEquipment%20Widget%20Ref _returnvalue_2))
          (UserInterface|Viewport|AddtoViewport _output_get_2 0)
          (Variables|/Script/Engine.PlayerController|SetbShowMouseCursor _returnvalue true))))))

(event EventBeginPlay
  (bind _owner (Class|BPIPlayerInterface|GetOwnerRef(Message) (Game|Player|GetPlayerPawn 0)))
  (bind _output_get (Variables|Default|SetOwner _owner))
  (bind _follow_camera (Class|BPIPlayerInterface|GetFollowCamera(Message) _output_get))
  (Variables|Refs|SetFollow%20Camera _follow_camera))

(fn EquipWeapon
  (params (Weapon%20Name :type Name))
  (bind _owner (Variables|Default|GetOwner))
  (Utilities|FlowControl|Sequence
    (:then_0
      (Variables|Default|SetWeapon%20Name Weapon%20Name)
      (Utilities|IsValid _owner
        (:Is%20Valid
          (bind _mesh (Class|BPIPlayerInterface|GetOwnerMesh(Message) _owner))
          (Variables|Default|SetMesh _mesh)
          (bind _weapon_socket_name (Class|BPIPlayerInterface|GetWeaponSocketRef(Message) _owner))
          (Variables|Default|SetWeapon%20Socket%20Name _weapon_socket_name)
          (bind _weapon_spawner (Class|BPIPlayerInterface|GetWeaponSpawnerRef(Message) _owner))
          (Variables|Default|SetWeapon%20Spawner _weapon_spawner))))
    (:then_1
      (bind _weapon_actor_ref (Class|BPIEquipment|SpawnActiveWeapon(Message) (Variables|Default|GetWeapon%20Spawner) (Transformation|GetSocketTransform (Variables|Default|GetMesh) (Variables|Default|GetWeapon%20Socket%20Name) "RTS_World") (Variables|Default|GetWeapon%20Name)))
      (bind _output_get (Variables|Default|SetSpawned%20Weapon _weapon_actor_ref))
      (Transformation|AttachComponentToComponent _output_get (Variables|Default|GetMesh) (Variables|Default|GetWeapon%20Socket%20Name) "SnapToTarget" "SnapToTarget" "SnapToTarget" true)
      (return (Variables|Default|GetSpawned%20Weapon)))))

(fn AddItemtoWeapons
  (params (New%20Weapon :type STX%20Weapons%20Structure%20%28by%20ref%29))
  (Development|PrintString "trying to add")
  (Utilities|Array|Add (Variables|Default|GetWeapon%20Slots) New%20Weapon)
  (Variables|Default|SetWeapon%20Name (.WeaponName (Utilities|Struct|BreakSTX_Weapons New%20Weapon)))
  (Development|PrintString "finished adding"))