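; Enemy combat ability actor that performs one step of a light attack combo.
; InitiateLightAttack caches the attacker, mesh and weapon via message calls, then sets reduced physical and elemental damage modifiers.
; Within combo length, it plays the weapon's montage for the current index and increments the enemy's index.
; Montage completion resets the index, ends the attack and destroys the actor; interruption and out-of-range indices skip this cleanup.
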(event Custom|Finish%20Attack
  (CallFunction|EndAttack)
  (Actor|DestroyActor))

(event EventInitiateLightAttack
  (params (Calling%20Actor :type Actor%20Object%20Reference) (Attack%20Index :type Integer) (Combo :type Boolean) (Punish :type Boolean))
  (CallFunction|StartAttack Calling%20Actor)
  (Variables|Default|SetPunish Punish)
  (Variables|Default|SetCombo Combo)
  (CallFunction|SetRefrenceVaraibles Calling%20Actor Attack%20Index "NewEnumerator0")
  (CallFunction|SetEnemyAbilityDamage 0.75 0.75)
  (if (not (>= (Variables|Default|GetAttack%20Index) (Variables|Default|GetLight%20Combo%20Length)))
    (bind _montage_to_play (Class|BPIWeapons|GetLightMonts(Message) (Variables|Reference|GetEnemy%20Weapon%20Ref) (Variables|Default|GetAttack%20Index)))
    (bind _result (Math|Integer|IncrementInt (Variables|Default|GetAttack%20Index))
      (:%20%20
        (Class|BPIEnemyInterface|SetAttackIndex(Message) (Variables|Default|GetOwning_Actor_ref) _result)
        (Animation|Montage|PlayMontage (Variables|Default|GetOwner_Mesh_ref) _montage_to_play
          (:then
            (Utilities|FlowControl|Delay 0.3))
          (:OnCompleted
            (Class|BPIEnemyInterface|SetAttackIndex(Message) (Variables|Default|GetOwning_Actor_ref))
            (CallFunction|FinishAttack)))))))

(fn ConstructionScript
  (|CallParentFunction))

(fn InitAttackState)

(fn CleanUpAttackState)

(fn SetRefrenceVaraibles
  (params (Attacker :type Actor%20Object%20Reference) (Attack%20Index :type Integer) (Attack%20Type :type ENUM_Enemy_Attack_types%20Enum :default "NewEnumerator0"))
  (bind _owner (Class|BPIEnemyInterface|GetOwnerEnemyRef(Message) Attacker))
  (Variables|Default|SetOwning_Actor_ref _owner)
  (bind _mesh (Class|BPIEnemyInterface|GetEnemyOwnerMesh(Message) (Variables|Default|GetOwning_Actor_ref)))
  (Variables|Default|SetOwner_Mesh_ref _mesh)
  (bind _equiped_weapon (Class|BPIEnemyInterface|GetEnemyWeaponRef(Message) (Variables|Default|GetOwning_Actor_ref)))
  (Variables|Reference|SetEnemy%20Weapon%20Ref _equiped_weapon)
  (Variables|Default|SetAttack%20Index Attack%20Index)
  (Variables|Default|SetAttack%20Type Attack%20Type))