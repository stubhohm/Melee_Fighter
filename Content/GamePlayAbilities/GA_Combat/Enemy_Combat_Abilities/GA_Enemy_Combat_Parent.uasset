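; Parent ability for enemy melee combat, managing attack state, combo data and weapon hit detection.
; Attack start and end update owner state through interface messages, and a helper scales the owner's attack ratings into ability damage.
; During trace windows, a looping timer sphere-traces from weapon base to tip, using DoOnce to limit repeated player damage.
; A montage macro advances the attack index but is unused in this graph.
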(event Custom|End%20Attack
  (Utilities|ResolveAttackDefaults))

(event Custom|Start_attack
  (params (Owning%20Actor :type Actor%20Object%20Reference))
  (bind _output_get (Variables|Default|SetOwning_Actor_ref Owning%20Actor))
  (Utilities|SetStartAttackDefaults _output_get))

(event Custom|Weapon%20Trace%20Loop
  ;[0 0 0] Weapon Tracing
  (bind (_base _tip) (Class|BPIWeapons|GetWeaponTipandBase(Message) (Variables|Default|GetEquiped%20Weapon)))
  (bind (_outhit _returnvalue) (Collision|SphereTraceByChannel _base _tip 12.0 "TraceTypeQuery1" false (Utilities|Array|MakeArray (Variables|Default|GetEquiped%20Weapon) (Variables|Default|GetOwning_Actor_ref)) "ForOneFrame"))
  (if _returnvalue
    (bind _is_player (Class|BPIPlayerInterface|IsPlayer(Message) (.HitActor (Collision|BreakHitResult _outhit))))
    (if _is_player
      (Variables|Reference|SetHit%20Actor (.HitActor (Collision|BreakHitResult _outhit)))
      (Utilities|FlowControl|DoOnce false :!label _label
        (:Completed
          (bind (_damage_type _element_type) (Class|BPIWeapons|GetWeaponAttributes(Message) (Variables|Default|GetEquiped%20Weapon)))
          (Class|BPIPlayerInterface|PlayerTakeDamage(Message) (Variables|Reference|GetHit%20Actor) (Variables|Default|GetOwning_Actor_ref) _damage_type (Variables|Attacking|GetPhysical%20Ability%20Damage) _element_type (Variables|Attacking|GetElemental%20Ability%20Damage))))
      (else
        (goto _label Reset)))))

(event EventRelayStartWeaponTrace
  (params (Self%20Ref :type Actor%20Object%20Reference) (Animation :type Anim%20Sequence%20Base%20Object%20Reference) (Weapon%20Ref :type Actor%20Object%20Reference))
  ;[0 0 0] Weapon Tracing
  (Variables|Default|SetOwning_Actor_ref Self%20Ref)
  (Variables|Attacking|SetAnimation Animation)
  (Variables|Default|SetEquiped%20Weapon Weapon%20Ref)
  (bind _returnvalue (Utilities|Time|SetTimerbyEvent (delegate Custom|Weapon%20Trace%20Loop) 0.01 true))
  (Variables|Tracing|SetWeapon%20Trace _returnvalue)
  (bind (_physical_ability_damage _elemental_ability_damage) (Class|BPIEnemyInterface|GetEnemyAbilityDamage(Message) (Variables|Default|GetOwning_Actor_ref)))
  (Variables|Attacking|SetPhysical%20Ability%20Damage _physical_ability_damage)
  (Variables|Attacking|SetElemental%20Ability%20Damage _elemental_ability_damage))

(event EventRelayEndWeaponTrace
  ;[0 0 0] Weapon Tracing
  (Utilities|Time|ClearandInvalidateTimerbyHandle (Variables|Tracing|GetWeapon%20Trace))
  (Utilities|FlowControl|DoOnce false) ; enters at Reset
)

(fn ConstructionScript
  (|CallParentFunction))

(fn SetEnemyAbilityDamage
  (params (Physical%20Damage%20Modifier :type Float%20%28double-precision%29) (Elemntal%20Damage%20Modifier :type Float%20%28double-precision%29))
  (bind (_physical_attack_rating _elemental_attack_rating) (Class|BPIEnemyInterface|GetEnemyAttackRatings(Message) (Variables|Default|GetOwning_Actor_ref)))
  (Class|BPIEnemyInterface|SetEnemyAbilityDamge(Message) (Variables|Default|GetOwning_Actor_ref) (* Physical%20Damage%20Modifier _physical_attack_rating) (* Elemntal%20Damage%20Modifier _elemental_attack_rating)))

(fn GetPatrolRoute
  (return 0))

(fn GetPatrolState
  (return false))

(fn InitiateLightAttack
  (params (Calling%20Actor :type Actor%20Object%20Reference) (Attack%20Index :type Integer) (Combo :type Boolean) (Punish :type Boolean))
  (return))

(fn IsEnemyDead
  (return false))

(fn SetPatrolling
  (params (is_patrolling :type Boolean))
  (return false))

(fn SpeedSelection
  (params (Speed :type ENUM_Movement_Speed%20Enum :default "NewEnumerator0"))
  (return 0.0))