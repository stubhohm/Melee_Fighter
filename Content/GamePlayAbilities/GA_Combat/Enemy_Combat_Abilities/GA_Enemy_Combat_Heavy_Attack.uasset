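; Enemy heavy attack ability, an actor that runs one heavy melee attack for the calling enemy.
; InitiateHeavyAttack caches the enemy, mesh and weapon references through message calls, then applies heavy damage modifiers.
; The weapon supplies the montage by attack index, or its heavy sprint montage when Punish is set.
; Montage completion ends the combo and destroys the actor, as does FinishAttack after ending the attack.
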(event Custom|Finish%20Attack
  (CallFunction|EndAttack)
  (Actor|DestroyActor))

(event Custom|Finish%20Combo
  (CallFunction|EndCombo)
  (Actor|DestroyActor))

(event EventInitiateHeavyAttack
  (params (Calling%20Actor :type Actor%20Object%20Reference) (Attack%20Index :type Integer) (Combo :type Boolean) (Punish :type Boolean))
  (CallFunction|StartAttack Calling%20Actor)
  (Variables|Default|SetPunish Punish)
  (CallFunction|SetRefrenceVaraibles Calling%20Actor Attack%20Index "NewEnumerator1")
  (CallFunction|SetEnemyAbilityDamage 1.25 1.25)
  (bind _montage_to_play (Class|BPIWeapons|GetHeavyMonts(Message) (Variables|Reference|GetEnemy%20Weapon%20Ref) (Variables|Default|GetAttack%20Index)))
  (if (Variables|Default|GetPunish)
    (bind _heavy_attack_sprint_montage (Class|BPIWeapons|GetHeavySprintAttack(Message) (Variables|Reference|GetEnemy%20Weapon%20Ref)))
    (Variables|Default|SetMontage%20to%20Play _heavy_attack_sprint_montage)
    (else
      (Variables|Default|SetMontage%20to%20Play _montage_to_play)))
  (Class|BPIEnemyInterface|SetAttackIndex(Message) (Variables|Default|GetOwning_Actor_ref) (Variables|Default|GetAttack%20Index))
  (Animation|Montage|PlayMontage (Variables|Default|GetOwner_Mesh_ref) (Variables|Default|GetMontage%20to%20Play)
    (:OnCompleted
      (CallFunction|FinishCombo))))

(fn ConstructionScript
  (|CallParentFunction))

(fn InitAttackState)

(fn CleanUpAttackState)

(fn SetRefrenceVaraibles
  (params (Attacker :type Actor%20Object%20Reference) (Attack%20Index :type Integer) (Attack%20Type :type ENUM_Enemy_Attack_types%20Enum :default "NewEnumerator0"))
  (bind _owner (Class|BPIEnemyInterface|GetOwnerEnemyRef(Message) Attacker))
  (Variables|Default|SetOwning_Actor_ref _owner)
  (bind _mesh (Class|BPIEnemyInterface|GetEnemyOwnerMesh(Message) (Variables|Default|GetOwning_Actor_ref)))
  (Variables|Default|SetOwner_Mesh_ref _mesh)
  (bind _equiped_weapon (Class|BPIEnemyInterface|GetEnemyWeaponRef(Message) (Variables|Default|GetOwning_Actor_ref)))
  (Variables|Reference|SetEnemy%20Weapon%20Ref _equiped_weapon)
  (Variables|Default|SetAttack%20Index Attack%20Index)
  (Variables|Default|SetAttack%20Type Attack%20Type))