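; Heavy attack combat ability that plays the equipped weapon's heavy attack montages as a combo of up to five steps.
; Activation boosts physical and elemental damage modifiers, and each combo continue advances the index, which wraps at the weapon's light attack combo length.
; A montage macro uses DoOnce and a short delay to gate repeat calls.
; Montage completion ends the attack and destroys the ability actor.
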(event Custom|End%20Heavy%20Attack
  (CallFunction|EndAttack)
  (Actor|DestroyActor))

(event Custom|Activate%20Heavy%20Attack
  (CallFunction|StartAttack)
  (CallFunction|SetAbilityDamage 1.25 1.25)
  (if (>= (Variables|Default|GetAttack%20Index) (Variables|/Game/Equipment/Wieldable/GI_Wieldable_Item.GI_Wieldable_Item_C|GetLight%20Attack%20Combo%20Length (Variables|Default|GetEquiped%20Weapon%20Ref)))
    (Variables|Default|SetAttack%20Index 0))
  (switch int (Variables|Default|GetAttack%20Index)
    (:0
      (Utilities|CallAttackMontage (Variables|/Game/Equipment/Wieldable/GI_Wieldable_Item.GI_Wieldable_Item_C|GetHeavy%20Attack%201%20Mont%20 (Variables|Default|GetEquiped%20Weapon%20Ref))))
    (:1
      (Utilities|CallAttackMontage (Variables|/Game/Equipment/Wieldable/GI_Wieldable_Item.GI_Wieldable_Item_C|GetHeavy%20Attack%202%20Mont (Variables|Default|GetEquiped%20Weapon%20Ref))))
    (:2
      (Utilities|CallAttackMontage (Variables|/Game/Equipment/Wieldable/GI_Wieldable_Item.GI_Wieldable_Item_C|GetHeavy%20Attack%203%20Mont (Variables|Default|GetEquiped%20Weapon%20Ref))))
    (:3
      (Utilities|CallAttackMontage (Variables|/Game/Equipment/Wieldable/GI_Wieldable_Item.GI_Wieldable_Item_C|GetHeavy%20Attack%204%20Mont (Variables|Default|GetEquiped%20Weapon%20Ref))))
    (:4
      (Utilities|CallAttackMontage (Variables|/Game/Equipment/Wieldable/GI_Wieldable_Item.GI_Wieldable_Item_C|GetHeavy%20Attack%205%20Mont (Variables|Default|GetEquiped%20Weapon%20Ref))))))

(event Custom|Continue%20Heavy%20Combo
  (Math|Integer|IncrementInt (Variables|Default|GetAttack%20Index)
    (:%20%20
      (if (>= (Variables|Default|GetAttack%20Index) (Variables|/Game/Equipment/Wieldable/GI_Wieldable_Item.GI_Wieldable_Item_C|GetLight%20Attack%20Combo%20Length (Variables|Default|GetEquiped%20Weapon%20Ref)))
        (Variables|Default|SetAttack%20Index 0))
      (switch int (Variables|Default|GetAttack%20Index)
        (:0
          (Utilities|CallAttackMontage (Variables|/Game/Equipment/Wieldable/GI_Wieldable_Item.GI_Wieldable_Item_C|GetHeavy%20Attack%201%20Mont%20 (Variables|Default|GetEquiped%20Weapon%20Ref))))
        (:1
          (Utilities|CallAttackMontage (Variables|/Game/Equipment/Wieldable/GI_Wieldable_Item.GI_Wieldable_Item_C|GetHeavy%20Attack%202%20Mont (Variables|Default|GetEquiped%20Weapon%20Ref))))
        (:2
          (Utilities|CallAttackMontage (Variables|/Game/Equipment/Wieldable/GI_Wieldable_Item.GI_Wieldable_Item_C|GetHeavy%20Attack%203%20Mont (Variables|Default|GetEquiped%20Weapon%20Ref))))
        (:3
          (Utilities|CallAttackMontage (Variables|/Game/Equipment/Wieldable/GI_Wieldable_Item.GI_Wieldable_Item_C|GetHeavy%20Attack%204%20Mont (Variables|Default|GetEquiped%20Weapon%20Ref))))
        (:4
          (Utilities|CallAttackMontage (Variables|/Game/Equipment/Wieldable/GI_Wieldable_Item.GI_Wieldable_Item_C|GetHeavy%20Attack%205%20Mont (Variables|Default|GetEquiped%20Weapon%20Ref))))))))

(fn ConstructionScript
  (|CallParentFunction))