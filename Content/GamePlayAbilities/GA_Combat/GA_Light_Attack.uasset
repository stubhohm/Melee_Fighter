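; Light attack ability actor that plays the player's equipped-weapon combo montages at reduced physical and elemental damage.
; Activation plays a sprint attack when sprinting, setting the combo index from the weapon, otherwise the montage for the current index.
; Continuing increments the index, wrapping at the weapon's combo length, through a DoOnce-gated, briefly delayed montage call.
; Montage completion ends the attack and destroys the actor, while interruption clears the player's CanContinueCombo flag.
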(event Custom|end%20light%20attack
  (CallFunction|EndAttack)
  (Actor|DestroyActor))

(event Custom|Activate%20Light%20Attack
  (Utilities|SprintAttack
    (:then
      _)
    (:else
      _))
  (CallFunction|StartAttack)
  (CallFunction|SetAbilityDamage 0.75 0.75)
  (if (Variables|Default|GetPerform%20Sprint%20Attack)
    (Variables|Default|SetPerform%20Sprint%20Attack false)
    (Utilities|CallAttackMontage (Variables|/Game/Equipment/Wieldable/GI_Wieldable_Item.GI_Wieldable_Item_C|GetLight%20Attack%20Sprint (Variables|/Game/Player/Blueprints/BP_Player_Character.BP_Player_Character_C|GetEquiped%20Weapon%20ref (Variables|Default|GetBP_Player_ref))))
    (else
      (if (>= (Variables|Default|GetAttack%20Index) (Variables|/Game/Equipment/Wieldable/GI_Wieldable_Item.GI_Wieldable_Item_C|GetLight%20Attack%20Combo%20Length (Variables|Default|GetEquiped%20Weapon%20Ref)))
        (Variables|Default|SetAttack%20Index 0))
      (switch int (Variables|Default|GetAttack%20Index)
        (:0
          (Utilities|CallAttackMontage (Variables|/Game/Equipment/Wieldable/GI_Wieldable_Item.GI_Wieldable_Item_C|GetLight%20Attack%201%20Mont (Variables|Default|GetEquiped%20Weapon%20Ref))))
        (:1
          (Utilities|CallAttackMontage (Variables|/Game/Equipment/Wieldable/GI_Wieldable_Item.GI_Wieldable_Item_C|GetLight%20Attack%202%20Mont (Variables|Default|GetEquiped%20Weapon%20Ref))))
        (:2
          (Utilities|CallAttackMontage (Variables|/Game/Equipment/Wieldable/GI_Wieldable_Item.GI_Wieldable_Item_C|GetLight%20Attack%203%20Mont (Variables|Default|GetEquiped%20Weapon%20Ref))))
        (:3
          (Utilities|CallAttackMontage (Variables|/Game/Equipment/Wieldable/GI_Wieldable_Item.GI_Wieldable_Item_C|GetLight%20Attack%204%20Mont (Variables|Default|GetEquiped%20Weapon%20Ref))))
        (:4
          (Utilities|CallAttackMontage (Variables|/Game/Equipment/Wieldable/GI_Wieldable_Item.GI_Wieldable_Item_C|GetLight%20Attack%205%20Mont (Variables|Default|GetEquiped%20Weapon%20Ref))))))))

(event Custom|Continue%20Light%20Combo
  (CallFunction|ContinueCombo)
  (Math|Integer|IncrementInt (Variables|Default|GetAttack%20Index)
    (:%20%20
      (if (>= (Variables|Default|GetAttack%20Index) (Variables|/Game/Equipment/Wieldable/GI_Wieldable_Item.GI_Wieldable_Item_C|GetLight%20Attack%20Combo%20Length (Variables|Default|GetEquiped%20Weapon%20Ref)))
        (Variables|Default|SetAttack%20Index 0))
      (switch int (Variables|Default|GetAttack%20Index)
        (:0
          (Utilities|CallAttackMontage (Variables|/Game/Equipment/Wieldable/GI_Wieldable_Item.GI_Wieldable_Item_C|GetLight%20Attack%201%20Mont (Variables|Default|GetEquiped%20Weapon%20Ref))))
        (:1
          (Utilities|CallAttackMontage (Variables|/Game/Equipment/Wieldable/GI_Wieldable_Item.GI_Wieldable_Item_C|GetLight%20Attack%202%20Mont (Variables|Default|GetEquiped%20Weapon%20Ref))))
        (:2
          (Utilities|CallAttackMontage (Variables|/Game/Equipment/Wieldable/GI_Wieldable_Item.GI_Wieldable_Item_C|GetLight%20Attack%203%20Mont (Variables|Default|GetEquiped%20Weapon%20Ref))))
        (:3
          (Utilities|CallAttackMontage (Variables|/Game/Equipment/Wieldable/GI_Wieldable_Item.GI_Wieldable_Item_C|GetLight%20Attack%204%20Mont (Variables|Default|GetEquiped%20Weapon%20Ref))))
        (:4
          (Utilities|CallAttackMontage (Variables|/Game/Equipment/Wieldable/GI_Wieldable_Item.GI_Wieldable_Item_C|GetLight%20Attack%205%20Mont (Variables|Default|GetEquiped%20Weapon%20Ref))))))))

(event Custom|End%20Light%20Combo
  (CallFunction|EndAttack)
  (Actor|DestroyActor))

(fn ConstructionScript
  (|CallParentFunction))