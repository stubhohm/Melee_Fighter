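; Parent combat ability that supplies shared combo state, montage playback and weapon hit detection for melee attacks.
; Start and end events set the player's attack flags, while a PerformAttack helper, uncalled here, plays a montage and advances the attack index.
; A looping timer sphere-traces between weapon tip and base, sending damage once per trace window.
; ContinueCombo, ResolveHit and GetWeaponRef are empty, and IsEnemy always returns false.
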(event Custom|End%20Attack
  (Utilities|ResolveAttackDefaults))

(event Custom|Start_attack
  (Utilities|SetStartAttackDefaults))

(event Custom|Start%20Weapon%20Trace
  (params (Animation :type Anim%20Sequence%20Base%20Object%20Reference))
  ;[0 0 0] Weapon Tracing
  (Variables|Default|SetAnimation Animation)
  (bind _returnvalue (Utilities|Time|SetTimerbyEvent (delegate Custom|Weapon%20Trace%20Loop) 0.01 true))
  (Variables|Default|SetWeapon%20Trace _returnvalue))

(event Custom|Weapon%20Trace%20Loop
  (bind _equiped_weapon_ref (Variables|Default|GetEquiped%20Weapon%20Ref))
  ;[0 0 0] Weapon Tracing
  (bind (_outhit _returnvalue) (Collision|SphereTraceByChannel (Transformation|GetWorldLocation (Variables|/Game/Equipment/Wieldable/GI_Wieldable_Item.GI_Wieldable_Item_C|GetWeapon%20Tip _equiped_weapon_ref)) (Transformation|GetWorldLocation (Variables|/Game/Equipment/Wieldable/GI_Wieldable_Item.GI_Wieldable_Item_C|GetWeapon%20Base _equiped_weapon_ref)) 12.0 "TraceTypeQuery1" false 0 "ForDuration"))
  (if _returnvalue
    (Utilities|FlowControl|DoOnce false
      (:Completed
        (bind _output_get (Variables|Default|SetHit%20Actor (.HitActor (Collision|BreakHitResult _outhit))))
        (Class|BPIDamage|TakeDamage(Message) _output_get (Variables|Default|GetBP_Player_ref) (Variables|Default|GetHit%20Actor) (Variables|/Game/Player/Blueprints/BP_Player_Character.BP_Player_Character_C|GetAbility%20Damage (Variables|Default|GetBP_Player_ref)))))))

(event Custom|End%20Weapon%20Trace
  (Utilities|Time|ClearandInvalidateTimerbyHandle (Variables|Default|GetWeapon%20Trace))
  (Utilities|FlowControl|DoOnce false) ; enters at Reset
)

(event Custom|Continue%20Combo)

(event Custom|End%20Combo
  (Utilities|ResolveAttackDefaults))

(fn ConstructionScript
  (|CallParentFunction))

(fn ResolveHit)

(fn GetWeaponRef)

(fn IsEnemy
  (return false))