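; Player heavy attack ability that applies boosted physical and elemental damage and plays montages supplied by the equipped weapon.
; A sprinting activation plays the weapon's sprint attack and sets the combo index from it; otherwise the indexed combo montage plays.
; Combo continuation advances the index, wrapping at the weapon's combo length.
; Montage completion, blend-out or notifies end the attack and destroy the ability actor, while interruption calls InteruptAttack.
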(event Custom|End%20Heavy%20Attack
  (CallFunction|EndPlayerAttack)
  (Actor|DestroyActor))

(event Custom|Activate%20Heavy%20Attack
  (params (Calling%20Actor :type Actor%20Object%20Reference))
  (CallFunction|StartAbility Calling%20Actor)
  (Utilities|SprintAttack)
  (CallFunction|StartPlayerAttack)
  (CallFunction|SetPlayerAbilityDamage 1.25 1.25)
  (if (Variables|Default|GetPerform%20Sprint%20Attack)
    (Variables|Default|SetPerform%20Sprint%20Attack false)
    (Utilities|CallAttackMontage (Variables|Default|GetMontage%20To%20Play))
    (else
      (bind _heavy_combo_length (Class|BPIWeapons|GetComboLength(Message) (Variables|Default|GetEquiped%20Weapon)))
      (if (>= (Variables|Default|GetAttack%20Index) _heavy_combo_length)
        (Variables|Default|SetAttack%20Index 0))
      (bind _montage_to_play (Class|BPIWeapons|GetHeavyMonts(Message) (Variables|Default|GetEquiped%20Weapon) (Variables|Default|GetAttack%20Index)))
      (Utilities|CallAttackMontage _montage_to_play))))

(event Custom|Continue%20Heavy%20Combo
  (CallFunction|ContinuePlayerAttackCombo)
  (Math|Integer|IncrementInt (Variables|Default|GetAttack%20Index)
    (:%20%20
      (bind _heavy_combo_length (Class|BPIWeapons|GetComboLength(Message) (Variables|Default|GetEquiped%20Weapon)))
      (if (>= (Variables|Default|GetAttack%20Index) _heavy_combo_length)
        (Variables|Default|SetAttack%20Index 0))
      (bind _montage_to_play (Class|BPIWeapons|GetHeavyMonts(Message) (Variables|Default|GetEquiped%20Weapon) (Variables|Default|GetAttack%20Index)))
      (Utilities|CallAttackMontage _montage_to_play))))

(fn ConstructionScript
  (|CallParentFunction))