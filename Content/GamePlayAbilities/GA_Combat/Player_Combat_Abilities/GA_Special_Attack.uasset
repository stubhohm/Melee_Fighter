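; Player combat ability that runs the special attack combo with boosted physical and elemental damage.
; Begin starts the ability and Continue advances the attack index, which wraps at the equipped weapon's special combo length.
; The weapon supplies each step's montage, played through a DoOnce-guarded macro.
; Blend out, interruption or montage notifies send the owner an end-combo message and end the attack; completion only ends the attack.
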(event Custom|End%20Special%20Attack
  (CallFunction|EndPlayerAttack))

(event EventBeginSpecialAttack
  (params (Player%20Ref :type Actor%20Object%20Reference))
  (CallFunction|StartAbility Player%20Ref)
  (CallFunction|StartPlayerAttack)
  (CallFunction|SetPlayerAbilityDamage 1.25 1.25)
  (bind _special_combo_length (Class|BPIWeapons|GetComboLength(Message) (Variables|Default|GetEquiped%20Weapon)))
  (if (>= (Variables|Default|GetAttack%20Index) _special_combo_length)
    (Variables|Default|SetAttack%20Index 0))
  (bind _montage_to_play (Class|BPIWeapons|GetSpecialMonts(Message) (Variables|Default|GetEquiped%20Weapon) (Variables|Default|GetAttack%20Index)))
  (Utilities|CallAttackMontage _montage_to_play))

(event EventContinueSpecialAttack
  (params (Player%20ref :type Actor%20Object%20Reference))
  (Math|Integer|IncrementInt (Variables|Default|GetAttack%20Index)
    (:%20%20
      (bind _special_combo_length (Class|BPIWeapons|GetComboLength(Message) (Variables|Default|GetEquiped%20Weapon)))
      (if (>= (Variables|Default|GetAttack%20Index) _special_combo_length)
        (Variables|Default|SetAttack%20Index 0))
      (bind _montage_to_play (Class|BPIWeapons|GetSpecialMonts(Message) (Variables|Default|GetEquiped%20Weapon) (Variables|Default|GetAttack%20Index)))
      (Utilities|CallAttackMontage _montage_to_play))))

(fn ConstructionScript
  (|CallParentFunction))

(fn GetAttackType
  (return "NewEnumerator3"))