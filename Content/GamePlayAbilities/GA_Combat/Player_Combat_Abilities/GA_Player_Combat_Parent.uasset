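; Parent player combat ability that handles attack state, combos and melee weapon damage.
; Start and end events set or reset owner states through message calls, while a helper macro plays attack montages and advances the combo index.
; Damage is attack ratings scaled by modifiers and stored on the owner.
; During trace windows, a fast looping timer sphere-traces from weapon base to tip and damages enemies, gated by a DoOnce that resets on non-enemy results.
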(event Custom|End%20Player%20Attack
  (Utilities|ResolveAttackDefaults))

(event Custom|Start%20Player%20attack
  (Utilities|SetStartAttackDefaults))

(event Custom|Interupt%20Attack
  ;[0 0 0] Turns off attack state if we are broken out of it
)

(event Custom|Weapon%20Trace%20Loop
  ;[0 0 0] Weapon Tracing
  (bind (_base _tip) (Class|BPIWeapons|GetWeaponTipandBase(Message) (Variables|Default|GetEquiped%20Weapon)))
  (bind _output_get (Variables|Default|SetAlready%20Hit (Utilities|Array|MakeArray (Variables|Default|GetOwning_Actor_ref) (Variables|Default|GetEquiped%20Weapon))))
  (bind _outhit (Collision|SphereTraceByChannel _base _tip 12.0 "TraceTypeQuery1" false _output_get "None" true "(R=1.000000,G=0.000000,B=0.000000,A=1.000000)" "(R=0.000000,G=1.000000,B=0.000000,A=1.000000)" 0.0))
  (bind _is_enemy (Class|BPIEnemyInterface|IsEnemy(Message) (.HitActor (Collision|BreakHitResult _outhit))))
  (if _is_enemy
    (Utilities|FlowControl|DoOnce false :!label _label
      (:Completed
        (Utilities|FlowControl|Sequence
          (:then_0
            (bind _output_get_2 (Variables|Default|SetHit%20Actor (.HitActor (Collision|BreakHitResult _outhit))))
            (bind (_damage_type _element_type) (Class|BPIWeapons|GetWeaponAttributes(Message) (Variables|Default|GetEquiped%20Weapon)))
            (Class|BPIPlayerCombat|EnemyTakeDamage(Message) _output_get_2 (Variables|Default|GetOwning_Actor_ref) (Variables|Default|GetHit%20Actor) _damage_type (Variables|Default|GetPhysical%20Ability%20Damage) _element_type (Variables|Default|GetElemental%20Ability%20Damage)))
          (:then_1
            (Utilities|Array|AppendArray (Utilities|Array|MakeArray (.HitActor (Collision|BreakHitResult _outhit))) (Variables|Default|GetAlready%20Hit))))))
    (else
      (goto _label Reset))))

(event Custom|Continue%20Player%20Attack%20Combo
  (Class|BPIPlayerInterface|ContinueCombo(Message) (Variables|Default|GetOwning_Actor_ref)))

(event Custom|End%20Player%20Attack%20Combo
  (Utilities|ResolveAttackDefaults))

(event EventRelayStartWeaponTrace
  (params (Self%20Ref :type Actor%20Object%20Reference) (Animation :type Anim%20Sequence%20Base%20Object%20Reference) (Weapon%20Ref :type Actor%20Object%20Reference))
  ;[0 0 0] Weapon Tracing
  (Variables|Default|SetAnimation Animation)
  (bind _returnvalue (Utilities|Time|SetTimerbyEvent (delegate Custom|Weapon%20Trace%20Loop) 0.01 true))
  (Variables|Default|SetWeapon%20Trace _returnvalue)
  (bind (_physical_ability_damage _elemental_ability_damage) (Class|BPIPlayerInterface|GetAbilityDamage(Message) (Variables|Default|GetOwning_Actor_ref)))
  (Variables|Default|SetPhysical%20Ability%20Damage _physical_ability_damage)
  (Variables|Default|SetElemental%20Ability%20Damage _elemental_ability_damage))

(event EventRelayEndWeaponTrace
  ;[0 0 0] Weapon Tracing
  (Utilities|Time|ClearandInvalidateTimerbyHandle (Variables|Default|GetWeapon%20Trace))
  (Variables|Default|SetAlready%20Hit (Variables|Default|GetEmpty%20Array))
  (Utilities|FlowControl|DoOnce false) ; enters at Reset
)

(fn ConstructionScript
  (|CallParentFunction))

(fn SetPlayerAbilityDamage
  (params (Physical%20Damage%20Modifier :type Float%20%28double-precision%29) (Elemntal%20Damage%20Modifier :type Float%20%28double-precision%29))
  (bind (_physical_attack_rating _elemental_attack_rating) (Class|BPIPlayerInterface|GetAttackRatings(Message) (Variables|Default|GetOwning_Actor_ref)))
  (Class|BPIPlayerInterface|SetAbilityDamge(Message) (Variables|Default|GetOwning_Actor_ref) (* Physical%20Damage%20Modifier _physical_attack_rating) (* Elemntal%20Damage%20Modifier _elemental_attack_rating)))

(fn GetAttackType
  (return "NewEnumerator4"))