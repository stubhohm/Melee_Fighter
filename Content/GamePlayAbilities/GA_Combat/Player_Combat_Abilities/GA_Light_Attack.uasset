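; Player light attack ability that plays the equipped weapon's light combo or sprint attack montages with reduced damage modifiers.
; On activation, a sprinting owner gets the weapon's sprint attack montage and combo index; otherwise the montage at the current index plays.
; Continue events advance the index, wrapping at combo length, through a DoOnce-gated, briefly delayed montage call.
; Montage completion ends the attack and destroys the ability actor, while interruption notifies the owner.
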(event Custom|end%20light%20attack
  (CallFunction|EndPlayerAttack)
  (Actor|DestroyActor))

(event Custom|Activate%20Light%20Attack
  (params (Calling%20Actor :type Actor%20Object%20Reference))
  (CallFunction|StartAbility Calling%20Actor)
  (Utilities|SprintAttack)
  (CallFunction|StartPlayerAttack)
  (CallFunction|SetPlayerAbilityDamage 0.75 0.75)
  (if (Variables|Default|GetPerform%20Sprint%20Attack)
    (Variables|Default|SetPerform%20Sprint%20Attack false)
    (Utilities|CallAttackMontage (Variables|Default|GetMontage%20To%20Play))
    (else
      (bind _light_combo_length (Class|BPIEquipment|GetComboLength(Message) (Variables|Default|GetEquiped%20Weapon)))
      (if (>= (Variables|Default|GetAttack%20Index) _light_combo_length)
        (Variables|Default|SetAttack%20Index 0))
      (bind _montage_to_play (Class|BPIEquipment|GetLightMonts(Message) (Variables|Default|GetEquiped%20Weapon) (Variables|Default|GetAttack%20Index)))
      (Utilities|CallAttackMontage _montage_to_play))))

(event Custom|Continue%20Light%20Combo
  (CallFunction|ContinuePlayerAttackCombo)
  (Math|Integer|IncrementInt (Variables|Default|GetAttack%20Index)
    (:%20%20
      (bind _light_combo_length (Class|BPIEquipment|GetComboLength(Message) (Variables|Default|GetEquiped%20Weapon)))
      (if (>= (Variables|Default|GetAttack%20Index) _light_combo_length)
        (Variables|Default|SetAttack%20Index 0))
      (bind _montage_to_play (Class|BPIEquipment|GetLightMonts(Message) (Variables|Default|GetEquiped%20Weapon) (Variables|Default|GetAttack%20Index)))
      (Utilities|CallAttackMontage _montage_to_play))))

(event Custom|End%20Light%20Combo
  (CallFunction|EndPlayerAttack)
  (Actor|DestroyActor))

(fn ConstructionScript
  (|CallParentFunction))