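; GA_Sprint is an ability actor that lets its owning character sprint at the cost of stamina.
; StartSprint raises walk speed and starts a looping drain timer if the owner is moving and not already sprinting; otherwise it clears the sprint state.
; Each drain decrements stamina through owner message calls, calling EndSprint when movement stops or stamina runs out.
; EndSprint restores walk speed, clears the timer and destroys the actor.
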(event Custom|End%20Sprint
  (bind _movement_component (Class|BPIPlayerInterface|GetMovementComponent(Message) (Variables|Default|GetOwning_Actor_ref)))
  (Variables|/Script/Engine.CharacterMovementComponent|SetMaxWalkSpeed _movement_component 5e+02)
  (Utilities|Time|ClearandInvalidateTimerbyHandle (Variables|Default|GetSprint%20Drain%20Timer))
  (Actor|DestroyActor))

(event Custom|Start%20Sprint
  (params (Calling%20Actor :type Actor%20Object%20Reference))
  (CallFunction|StartAbility Calling%20Actor)
  (bind _sprint_state (Class|BPIPlayerInterface|GetSprintState(Message) (Variables|Default|GetOwning_Actor_ref)))
  (if (and (not _sprint_state) (not (Utilities|Operators|EqualEqual :A (Variables|/Script/Engine.MovementComponent|GetVelocity (Variables|Default|GetMovement%20Component)) :ErrorTolerance 5.0)))
    (Class|BPIPlayerInterface|SetSprintState(Message) (Variables|Default|GetOwning_Actor_ref) true)
    (Variables|/Script/Engine.CharacterMovementComponent|SetMaxWalkSpeed (Variables|Default|GetMovement%20Component) 8.5e+02)
    (bind _returnvalue (Utilities|Time|SetTimerbyFunctionName 0 (Variables|Default|GetSprint%20Consumption%20Name) 0.075 true))
    (Variables|Default|SetSprint%20Drain%20Timer _returnvalue)
    (else
      (Class|BPIPlayerInterface|SetSprintState(Message) (Variables|Default|GetOwning_Actor_ref) false))))

(fn ConstructionScript
  (|CallParentFunction))

(fn SprintStaminaConsumption
  (bind _owning_actor_ref (Variables|Default|GetOwning_Actor_ref))
  (bind _stamina_points (Class|BPIPlayerInterface|GetHP,Stamina,andManaPoints(Message) (Variables|Default|GetOwning_Actor_ref)))
  (bind _result (Math|Float|DecrementFloat _stamina_points)
    (:%20%20
      (Class|BPIPlayerInterface|SetStaminaPoints(Message) _owning_actor_ref _result)
      (bind _movement_component (Class|BPIPlayerInterface|GetMovementComponent(Message) _owning_actor_ref))
      (LocalVariables|SetMovement%20Component _movement_component)
      (if (or (Utilities|Operators|EqualEqual :A (Variables|/Script/Engine.MovementComponent|GetVelocity (LocalVariables|GetMovement%20Component)) :ErrorTolerance 5.0) (<= _result 0.0))
        (CallFunction|EndSprint)))))