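; GA_Base_Ability is a base gameplay ability Blueprint that caches references to its owning actor and that actor's components.
; InitAbilities passes the player through GetActorRef to StartAbility, which stores the equipped weapon, movement component and owner mesh.
; References are fetched through interface messages, avoiding casts to concrete classes.
; The remaining functions, covering states, stats, damage and resources, are stubs returning empty or default values.
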(event Custom|Init%20Abilities
  (params (Player :type Actor%20Object%20Reference))
  (Reference|GetActorRef Player))

(event EventBeginPlay)

(fn ConstructionScript)

(fn GetActorRef
  (params (Player :type Actor%20Object%20Reference))
  (bind _owner (Class|BPIPlayerInterface|GetOwnerRef(Message) Player))
  (bind _output_get (Variables|Reference|SetOwning_Actor_ref _owner))
  (CallFunction|StartAbility _output_get))

(fn StartAbility
  (params (Calling%20Actor :type Actor%20Object%20Reference))
  (Variables|Reference|SetOwning_Actor_ref Calling%20Actor)
  (bind _equiped_weapon (Class|BPIPlayerInterface|GetWeaponRef(Message) (Variables|Reference|GetOwning_Actor_ref)))
  (Variables|Reference|SetEquiped%20Weapon _equiped_weapon)
  (bind _movement_component (Class|BPIPlayerInterface|GetMovementComponent(Message) (Variables|Reference|GetOwning_Actor_ref)))
  (Variables|Default|SetMovement%20Component _movement_component)
  (bind _mesh (Class|BPIPlayerInterface|GetOwnerMesh(Message) (Variables|Reference|GetOwning_Actor_ref)))
  (Variables|Reference|SetOwner_Mesh_ref _mesh))

(fn GetCrouchStae
  (return false))

(fn GetSprintState
  (return false))

(fn GetAbilityDamage
  (return 0.0 0.0))

(fn GetMaxStats
  (return 0.0 0.0 0.0 0 0 0 0))

(fn GetOwnerMesh
  (return 0))

(fn GetRelativeMovementDirection
  (return ""))

(fn GetDodgeState
  (return false))

(fn GetAttackState
  (return false))

(fn GetLockon
  (return false))

(fn SetStaminaPoints
  (params (Stamina%20Points :type Float%20%28double-precision%29))
  (return))

(fn GetHP,Stamina,andManaPoints
  (return 0.0 0.0 0.0))

(fn GetMovementComponent
  (return 0))

(fn GetAttackRatings
  (return 0.0 0.0))

(fn GetWeaponRef
  (return 0))

(fn GetOwnerRef
  (return 0))